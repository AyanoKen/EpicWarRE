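; BP_Altar is a capturable altar that periodically boosts every unit of the team holding it.
; The first overlapping BP_ParentUnit becomes master, setting the team material and starting a looping timer, apparently for UseAltarMagic.
; Depending on AltarType, that event either permanently adds stacking Damage or restores clamped HP to same-team units.
; When the master leaves, the altar reverts to neutral and clears the timer, without checking for units still inside.
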(event `self.Collider.OnComponentBeginOverlap`
  (params (OverlappedComponent :type "PrimitiveComponent Object Reference") (OtherActor :type "Actor Object Reference") (OtherComp :type "PrimitiveComponent Object Reference") (OtherBodyIndex :type Integer) (bFromSweep :type Boolean) (SweepResult :type "HitResult Structure (by ref)"))
  (bind _asbp_parent_unit (cast `/Game/MyGame/Blueprints/BP_ParentUnit` OtherActor))
  (if (not (`KismetSystemLibrary.IsValid` (`self.CurretMaster`)))
    (bind _output_get (set `self.CurretMaster` _asbp_parent_unit))
    (bind _output_get_2 (set `self.CurrentTeam` (`/Game/MyGame/Blueprints/BP_ParentUnit.TeamID` _output_get)))
    (`PrimitiveComponent.SetMaterial` (`self.StaticMesh`) 0 (`|GetArrayItem` (`self.TeamMaterials`) _output_get_2))
    (`KismetSystemLibrary.K2_ClearAndInvalidateTimerHandle` (`self.MagicTimer`))
    (bind _returnvalue (`KismetSystemLibrary.K2_SetTimerDelegate` (`|CreateDelegate` :!event `UseAltarMagic`) 40.0 true))
    (set `self.MagicTimer` _returnvalue)))

(event `self.Collider.OnComponentEndOverlap`
  (params (OverlappedComponent :type "PrimitiveComponent Object Reference") (OtherActor :type "Actor Object Reference") (OtherComp :type "PrimitiveComponent Object Reference") (OtherBodyIndex :type Integer))
  (bind _asbp_parent_unit (cast `/Game/MyGame/Blueprints/BP_ParentUnit` OtherActor))
  (if (`KismetSystemLibrary.IsValid` (`self.CurretMaster`))
    (if (== _asbp_parent_unit (`self.CurretMaster`))
      (set `self.CurretMaster` null :!label _label)
      (bind _output_get (set `self.CurrentTeam` 2))
      (`PrimitiveComponent.SetMaterial` (`self.StaticMesh`) 0 (`|GetArrayItem` (`self.TeamMaterials`) _output_get))
      (`KismetSystemLibrary.K2_ClearAndInvalidateTimerHandle` (`self.MagicTimer`)))
    (else
      (goto _label))))

(event `UseAltarMagic`
  (`KismetSystemLibrary.PrintString` "Using Altar Magic")
  (switch `/Game/MyGame/Data/Enum_AltarTypes` (`self.AltarType`)
    (:`NewEnumerator0`
      (bind _outactors (`GameplayStatics.GetAllActorsOfClass` "/Game/MyGame/Blueprints/BP_ParentUnit.BP_ParentUnit_C"))
      (for _array_element _outactors
        (if (== (`/Game/MyGame/Blueprints/BP_ParentUnit.TeamID` _array_element) (`self.CurrentTeam`))
          (set `/Game/MyGame/Blueprints/BP_ParentUnit.Damage` (+ (`/Game/MyGame/Blueprints/BP_ParentUnit.Damage` _array_element) 20) _array_element))))
    (:`NewEnumerator1`
      (bind _outactors_2 (`GameplayStatics.GetAllActorsOfClass` "/Game/MyGame/Blueprints/BP_ParentUnit.BP_ParentUnit_C"))
      (for _array_element_2 _outactors_2
        (if (== (`/Game/MyGame/Blueprints/BP_ParentUnit.TeamID` _array_element_2) (`self.CurrentTeam`))
          (set `/Game/MyGame/Blueprints/BP_ParentUnit.CurrentHp` (`KismetMathLibrary.Clamp` (+ (`/Game/MyGame/Blueprints/BP_ParentUnit.CurrentHp` _array_element_2) 50) 0 (`/Game/MyGame/Blueprints/BP_ParentUnit.MaxHp` _array_element_2)) _array_element_2))))))

(fn `UserConstructionScript`)