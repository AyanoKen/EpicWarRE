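; Unit spawner that periodically spawns team units from its SpawnData, up to a cap.
; After a short BeginPlay delay, a looping timer drives spawning; upgrade level linearly scales the unit cap, damage and max HP.
; Each spawn gets team and stats, then after a delay repositions, updates its HP indicator and joins SpawnedUnits.
; At the cap, ArrayCleanup removes invalid entries and allows a spawn if any were removed.
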(event `self.ReceiveBeginPlay`
  (bind (_spawndata_unitclass _spawndata_spawninterval) (break `/Game/MyGame/Data/ST_UnitData_Main` (`self.SpawnData`)))
  (`KismetSystemLibrary.Delay` 2.0)
  (`KismetSystemLibrary.K2_SetTimerDelegate` (`|CreateDelegate` :!event `SpawnUnit`) _spawndata_spawninterval true))

(event `SpawnUnit`
  (bind (_spawndata_unitclass _spawndata_spawninterval _spawndata_maxunits _spawndata_maxhp _spawndata_damage _spawndata_teamid _spawndata_spawntransform _spawndata_texture _spawndata_upgradelevel) (break `/Game/MyGame/Data/ST_UnitData_Main` (`self.SpawnData`)))
  (bind _returnvalue (* (`KismetMathLibrary.Conv_IntToDouble` _spawndata_upgradelevel) 0.25))
  (if (> (+ _spawndata_maxunits (* (`KismetMathLibrary.Conv_IntToDouble` _spawndata_maxunits) _returnvalue)) (`KismetArrayLibrary.Array_Length` (`self.SpawnedUnits`)))
    (bind _returnvalue_2 (`|SpawnActorFromClass` _spawndata_unitclass _spawndata_spawntransform "DontSpawnIfColliding" "MultiplyWithRoot" null null :!label _label))
    (set `/Game/MyGame/Blueprints/BP_ParentUnit.TeamID` _spawndata_teamid _returnvalue_2)
    (set `/Game/MyGame/Blueprints/BP_ParentUnit.Damage` (+ _spawndata_damage (* (`KismetMathLibrary.Conv_IntToDouble` _spawndata_damage) _returnvalue)) _returnvalue_2)
    (bind _output_get (set `/Game/MyGame/Blueprints/BP_ParentUnit.MaxHp` (+ _spawndata_maxhp (* (`KismetMathLibrary.Conv_IntToDouble` _spawndata_maxhp) _returnvalue)) _returnvalue_2))
    (set `/Game/MyGame/Blueprints/BP_ParentUnit.CurrentHp` _output_get _returnvalue_2)
    (`KismetSystemLibrary.Delay` 1.0)
    (`/Game/MyGame/Blueprints/BP_ParentUnit.Reposition` _returnvalue_2)
    (`/Game/MyGame/Blueprints/BP_ParentUnit.ChangeHpIndicator` _returnvalue_2)
    (`KismetArrayLibrary.Array_Add` (`self.SpawnedUnits`) _returnvalue_2)
    (else
      (bind _madespace_ (`self.ArrayCleanup`))
      (if _madespace_
        (goto _label)))))

(fn `ArrayCleanup`
  (returns (`MadeSpace?` :type Boolean))
  (locals (RemovedCount :type Integer))
  (bind _spawnedunits (`self.SpawnedUnits`))
  (set `local.RemovedCount` 0)
  (for _array_element _spawnedunits
    (if (not (`KismetSystemLibrary.IsValid` _array_element))
      (bind _returnvalue (`KismetArrayLibrary.Array_RemoveItem` _spawnedunits _array_element))
      (if _returnvalue
        (`/Engine/EditorBlueprintResources/StandardMacros.IncrementInt` (`local.RemovedCount`)))))
  (if (> (`local.RemovedCount`) 0)
    (return true)
    (else
      (return false))))

(fn `UserConstructionScript`)