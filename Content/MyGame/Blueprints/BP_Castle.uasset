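; Team castle for a battle level that spawns unit spawners from GameInstance spawn data and serves as the win/lose objective.
; The enemy side starts looping timers, and its AI event briefly toggles the doors while sending idle units to the player anchor.
; Clicking the player castle toggles door collision and visibility.
; Damage updates HUD health bars; destruction awards gold, shows victory or defeat, then returns to ConquestScreen.
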(event `self.ReceiveBeginPlay`
  ;[0.15 0.15 0.15 0.5 42] Initialize
  (if (!= (`self.TeamId`) 0)
    (bind _asbp_game_instance (cast `/Game/MyGame/GameMode/BP_GameInstance` (`GameplayStatics.GetGameInstance`)))
    (bind _enemyspawndata (`/Game/MyGame/GameMode/BP_GameInstance.EnemySpawnData` _asbp_game_instance))
    (bind _outrownames (`DataTableFunctionLibrary.GetDataTableRowNames` _enemyspawndata))
    (for _array_element _outrownames
      (bind _returnvalue (`|GetDataTableRow` _enemyspawndata _array_element)
        (:`then`
          (bind _returnvalue_2 (`|SpawnActorFromClass` "/Game/MyGame/Blueprints/BP_UnitSpawner.BP_UnitSpawner_C" (`self.GetTransform`) "Undefined" "MultiplyWithRoot" null null))
          (set `/Game/MyGame/Blueprints/BP_UnitSpawner.SpawnData` _returnvalue _returnvalue_2)
          (`KismetSystemLibrary.K2_SetTimerDelegate` (`|CreateDelegate` :!event `EnemyAI`) 10.0 true))))
    (else
      (bind _asbp_game_instance_2 (cast `/Game/MyGame/GameMode/BP_GameInstance` (`GameplayStatics.GetGameInstance`)))
      (for _array_element_2 (`/Game/MyGame/GameMode/BP_GameInstance.PlayerSpawnData` _asbp_game_instance_2)
        (bind _returnvalue_3 (`|SpawnActorFromClass` "/Game/MyGame/Blueprints/BP_UnitSpawner.BP_UnitSpawner_C" (`self.GetTransform`) "Undefined" "MultiplyWithRoot" null null))
        (set `/Game/MyGame/Blueprints/BP_UnitSpawner.SpawnData` _array_element_2 _returnvalue_3)))))

(event `EnemyAI`
  ;[0.15 0.15 0.15 0.5 42] Enemy AI
  (`self.ToggleDoors`)
  (bind _outactors (`GameplayStatics.GetAllActorsOfClass` "/Game/MyGame/Blueprints/BP_ParentUnit.BP_ParentUnit_C"))
  (for _array_element _outactors
    (if (and (== (`/Game/MyGame/Blueprints/BP_ParentUnit.TeamID` _array_element) 1) (not (`/Game/MyGame/Blueprints/BP_ParentUnit.IsInBattle?` _array_element)))
      (`/Game/MyGame/Blueprints/BP_ParentUnit.MoveToLocation` _array_element (`self.K2_GetActorLocation` (`self.Anchor_Player`)))))
  (`KismetSystemLibrary.Delay` 5.0)
  (`self.ToggleDoors`))

(event `self.ReceiveActorOnClicked`
  (params (ButtonPressed :type "Key Structure"))
  ;[0.15 0.15 0.15 0.5 42] Click Castle
  (if (== (`self.TeamId`) 0)
    (`self.ToggleDoors`)))

(event `TakeDamage`
  (params (Damage :type Integer))
  (bind _castlehp (`self.CastleHp`))
  ;[0.15 0.15 0.15 0.5 42] Damage
  (if (not (`KismetSystemLibrary.IsValid` (`self.HUD`)))
    (bind _asbp_player_controller (cast `/Game/MyGame/Blueprints/BP_PlayerController` (`GameplayStatics.GetPlayerController` 0)))
    (set `self.HUD` (`/Game/MyGame/Blueprints/BP_PlayerController.HUD` _asbp_player_controller)))
  (if (not (<= _castlehp 0))
    (bind _output_get (set `self.CastleHp` (- _castlehp Damage)))
    (`self.UpdateProgressBars`)
    (if (<= _output_get 0)
      (bind _asbp_game_instance (cast `/Game/MyGame/GameMode/BP_GameInstance` (`GameplayStatics.GetGameInstance`)))
      (switch `int` (`self.TeamId`)
        (:`0`
          (bind _playergold (`/Game/MyGame/GameMode/BP_GameInstance.PlayerGold` _asbp_game_instance))
          (set `/Game/MyGame/GameMode/BP_GameInstance.PlayerGold` (+ _playergold 5000) _asbp_game_instance)
          (bind _returnvalue (`|CreateWidget` "/Game/MyGame/UI/WBP_Defeat.WBP_Defeat_C" (`GameplayStatics.GetPlayerController` 0)))
          (`UserWidget.AddToViewport` _returnvalue 0)
          (`KismetSystemLibrary.Delay` 5.0)
          (`GameplayStatics.OpenLevel` "ConquestScreen"))
        (:`1`
          (set `/Game/MyGame/GameMode/BP_GameInstance.PlayerGold` (+ _playergold 20000) _asbp_game_instance)
          (bind _returnvalue_2 (`|CreateWidget` "/Game/MyGame/UI/WBP_Victory.WBP_Victory_C" (`GameplayStatics.GetPlayerController` 0)))
          (`UserWidget.AddToViewport` _returnvalue_2 0)
          (bind _asbp_game_instance_2 (cast `/Game/MyGame/GameMode/BP_GameInstance` (`GameplayStatics.GetGameInstance`)))
          (set `/Game/MyGame/GameMode/BP_GameInstance.ConquestResult` 1 _asbp_game_instance_2)
          (`KismetSystemLibrary.Delay` 5.0)
          (`GameplayStatics.OpenLevel` "ConquestScreen"))))))

(fn `SpawnUnit`)

(fn `ToggleDoors`
  (bind _door1 (`self.Door1`))
  (bind _door2 (`self.Door2`))
  (bind _door1_2 (`self.Door1`))
  (bind _door2_2 (`self.Door2`))
  (if (`self.AreDoorsOpen?`)
    (`PrimitiveComponent.SetCollisionProfileName` _door1_2 "BlockAll" true)
    (`SceneComponent.SetVisibility` _door1_2 true false)
    (`PrimitiveComponent.SetCollisionProfileName` _door2_2 "BlockAll" true)
    (`SceneComponent.SetVisibility` _door2_2 true false)
    (set `self.AreDoorsOpen?` false)
    (else
      (`PrimitiveComponent.SetCollisionProfileName` _door1 "OverlapAll" true)
      (`SceneComponent.SetVisibility` _door1 false false)
      (`PrimitiveComponent.SetCollisionProfileName` _door2 "OverlapAll" true)
      (`SceneComponent.SetVisibility` _door2 false false)
      (set `self.AreDoorsOpen?` true))))

(fn `UpdateProgressBars`
  (bind _returnvalue (/ (`KismetMathLibrary.Conv_IntToDouble` (`self.CastleHp`)) (`KismetMathLibrary.Conv_IntToDouble` (`self.CastleMaxHp`))))
  (switch `int` (`self.TeamId`)
    (:`0`
      (bind _aswbp_hud (cast `/Game/MyGame/UI/WBP_HUD` (`self.HUD`)))
      (`ProgressBar.SetPercent` (`/Game/MyGame/UI/WBP_HUD.PlayerHP` _aswbp_hud) _returnvalue))
    (:`1`
      (bind _aswbp_hud_2 (cast `/Game/MyGame/UI/WBP_HUD` (`self.HUD`)))
      (`ProgressBar.SetPercent` (`/Game/MyGame/UI/WBP_HUD.EnemyHP` _aswbp_hud_2) _returnvalue))))

(fn `UserConstructionScript`
  (set `self.CastleMaxHp` (`self.CastleHp`)))