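; BP_CameraPawn is a player-controlled camera pawn that pans over the level within a fixed rectangular area.
; Enhanced Input move actions apply forward and right movement input and cancel any active camera glide.
; Every tick it clamps X and Y to the bounds.
; While the TeleportCamera flag is set, it interpolates smoothly toward TargetLocation, clearing the flag on arrival.
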(event `self.ReceiveTick`
  (params (DeltaSeconds :type "Float (single-precision)"))
  (bind _returnvalue (`self.K2_GetActorLocation`))
  (bind _targetlocation (`self.TargetLocation`))
  (`self.CheckCameraBounds`)
  (if (`self.TeleportCamera`)
    (if (> (`KismetMathLibrary.Vector_Distance` _returnvalue _targetlocation) 5.0)
      (`self.K2_SetActorLocation` (`KismetMathLibrary.VInterpTo` _returnvalue _targetlocation DeltaSeconds 5.0))
      (else
        (set `self.TeleportCamera` false)))))

(event `EnhancedInput|/Game/MyGame/Input/IA_MoveForward`
  (params (ActionValue :type "Float (double-precision)") (ElapsedSeconds :type "Float (double-precision)") (TriggeredSeconds :type "Float (double-precision)") (InputAction :type "InputAction Object Reference" :default "/Game/MyGame/Input/IA_MoveForward.IA_MoveForward"))
  (:`Triggered`
    (set `self.TeleportCamera` false)
    (`self.AddMovementInput` (`self.GetActorForwardVector`) ActionValue)))

(event `EnhancedInput|/Game/MyGame/Input/IA_MoveRight`
  (params (ActionValue :type "Float (double-precision)") (ElapsedSeconds :type "Float (double-precision)") (TriggeredSeconds :type "Float (double-precision)") (InputAction :type "InputAction Object Reference" :default "/Game/MyGame/Input/IA_MoveRight.IA_MoveRight"))
  (:`Triggered`
    (set `self.TeleportCamera` false)
    (`self.AddMovementInput` (`self.GetActorRightVector`) ActionValue)))

(fn `CheckCameraBounds`
  (bind (_returnvalue_x _returnvalue_y _returnvalue_z) (`KismetMathLibrary.BreakVector` (`self.K2_GetActorLocation`)))
  (`self.K2_SetActorLocation` (`KismetMathLibrary.MakeVector` (`KismetMathLibrary.FClamp` _returnvalue_x -4400.0 4400.0) (`KismetMathLibrary.FClamp` _returnvalue_y -4000.0 4000.0) _returnvalue_z)))

(fn `UserConstructionScript`)