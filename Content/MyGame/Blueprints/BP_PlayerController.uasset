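; RTS-style player controller for selecting team 0 units and ordering them to move.
; Left click selects one unit under the cursor, while Ctrl-drag resizes a selection box widget each tick and selects units whose screen-projected positions fall inside it.
; An event also adds every team 0 unit of a given class to the selection.
; The set-destination click spawns a cursor effect and moves the multi-selection, or else the single selected unit.
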(event `self.ReceiveBeginPlay`
  (bind _returnvalue (pcsubsystem `EnhancedInputLocalPlayerSubsystem` (`GameplayStatics.GetPlayerController` 0)))
  (`EnhancedInputSubsystemInterface.AddMappingContext` _returnvalue "/Game/TopDown/Input/IMC_Default.IMC_Default" 0 (struct))
  (`EnhancedInputSubsystemInterface.AddMappingContext` _returnvalue "/Game/MyGame/Input/IMC_Camera.IMC_Camera" 0 (struct)))

(event `SelectAllUnitsOfClass`
  (params (Class :type "/Game/MyGame/Blueprints/BP_ParentUnit Class Reference"))
  (bind _outactors (`GameplayStatics.GetAllActorsOfClass` Class))
  (for _array_element _outactors
    (bind _asbp_parent_unit (cast `/Game/MyGame/Blueprints/BP_ParentUnit` _array_element))
    (if (== (`/Game/MyGame/Blueprints/BP_ParentUnit.TeamID` _asbp_parent_unit) 0)
      (`/Game/MyGame/Blueprints/BP_ParentUnit.Toggle Selection` _asbp_parent_unit true)
      (`KismetArrayLibrary.Array_AddUnique` (`self.MultiSelectUnits`) _asbp_parent_unit))))

(event `EnhancedInput|/Game/TopDown/Input/Actions/IA_SetDestination_Click`
  (params (ActionValue :type Boolean) (ElapsedSeconds :type "Float (double-precision)") (TriggeredSeconds :type "Float (double-precision)") (InputAction :type "InputAction Object Reference" :default "/Game/TopDown/Input/Actions/IA_SetDestination_Click.IA_SetDestination_Click"))
  (bind _selectedunit (`self.SelectedUnit`))
  (:`Triggered`
    (`NiagaraFunctionLibrary.SpawnSystemAtLocation` "/Game/Cursor/FX_Cursor.FX_Cursor" (`.Location` (`GameplayStatics.BreakHitResult` (`self.GetHitResultUnderCursorByChannel` "TraceTypeQuery1"))))
    (if (`KismetArrayLibrary.Array_IsNotEmpty` (`self.MultiSelectUnits`))
      (for _array_element (`self.MultiSelectUnits`)
        (if (`KismetSystemLibrary.IsValid` _array_element)
          (`/Game/MyGame/Blueprints/BP_ParentUnit.MoveToLocation` _array_element (`.Location` (`GameplayStatics.BreakHitResult` (`self.GetHitResultUnderCursorByChannel` "TraceTypeQuery1"))))))
      (elif (`KismetSystemLibrary.IsValid` _selectedunit)
        (`/Game/MyGame/Blueprints/BP_ParentUnit.MoveToLocation` _selectedunit (`.Location` (`GameplayStatics.BreakHitResult` (`self.GetHitResultUnderCursorByChannel` "TraceTypeQuery1"))))))))

(event `Key|LeftMouseButton`
  (params (Key :type "Key Structure"))
  (:`Pressed`
    (`self.ClearSelection`)
    (if (`self.IsInputKeyDown` "LeftControl")
      (set `self.IsDragging?` true)
      (bind _returnvalue (`WidgetLayoutLibrary.GetMousePositionOnViewport`))
      (set `self.DragStartPos` (`KismetMathLibrary.MakeVector2D` (`KismetMathLibrary.BreakVector2D` _returnvalue) (`.Y` (`KismetMathLibrary.BreakVector2D` _returnvalue))))
      (bind _returnvalue_2 (`|CreateWidget` "/Game/MyGame/UI/WBP_SelectionBox.WBP_SelectionBox_C" self))
      (`UserWidget.AddToViewport` _returnvalue_2 0)
      (set `self.SelectionBox` _returnvalue_2)
      (else
        (`self.SelectSingleTarget`))))
  (:`Released`
    (if (`self.IsDragging?`)
      (set `self.IsDragging?` false)
      (`Widget.RemoveFromParent` (`self.SelectionBox`))
      (set `self.SelectionBox` null)
      (`self.SelectMultiTarget`))))

(event `self.ReceiveTick`
  (params (DeltaSeconds :type "Float (single-precision)"))
  (bind (_dragstartpos_x _dragstartpos_y) (`KismetMathLibrary.BreakVector2D` (`self.DragStartPos`)))
  (bind (_dragstartpos_x_2 _dragstartpos_y_2) (`KismetMathLibrary.BreakVector2D` (`self.DragStartPos`)))
  (bind (_dragendpos_x _dragendpos_y) (`KismetMathLibrary.BreakVector2D` (`self.DragEndPos`)))
  (bind _returnvalue (`WidgetLayoutLibrary.SlotAsCanvasSlot` (`/Game/MyGame/UI/WBP_SelectionBox.SelectionPanel` (`self.SelectionBox`))))
  (if (`self.IsDragging?`)
    (bind _returnvalue_2 (`WidgetLayoutLibrary.GetMousePositionOnViewport`))
    (bind _output_get (set `self.DragEndPos` (`KismetMathLibrary.MakeVector2D` (`KismetMathLibrary.BreakVector2D` _returnvalue_2) (`.Y` (`KismetMathLibrary.BreakVector2D` _returnvalue_2)))))
    (`CanvasPanelSlot.SetSize` _returnvalue (`KismetMathLibrary.MakeVector2D` (- (`KismetMathLibrary.BreakVector2D` _output_get) _dragstartpos_x) (- (`.Y` (`KismetMathLibrary.BreakVector2D` _output_get)) _dragstartpos_y)))
    (`CanvasPanelSlot.SetPosition` _returnvalue (`KismetMathLibrary.MakeVector2D` (`KismetMathLibrary.FMin` _dragstartpos_x_2 _dragendpos_x) (`KismetMathLibrary.FMin` _dragstartpos_y_2 _dragendpos_y)))))

(fn `ClearSelection`
  (bind _selectedunit (`self.SelectedUnit`))
  (bind _multiselectunits (`self.MultiSelectUnits`))
  (`|ExecutionSequence`
    (:`then_0`
      (if (`KismetSystemLibrary.IsValid` _selectedunit)
        (`/Game/MyGame/Blueprints/BP_ParentUnit.Toggle Selection` _selectedunit false)
        (set `self.SelectedUnit` null)))
    (:`then_1`
      (if (`KismetArrayLibrary.Array_IsNotEmpty` (`self.MultiSelectUnits`))
        (for _array_element _multiselectunits
          (if (`KismetSystemLibrary.IsValid` _array_element)
            (`/Game/MyGame/Blueprints/BP_ParentUnit.Toggle Selection` _array_element false)))
        (`KismetArrayLibrary.Array_Clear` _multiselectunits)))))

(fn `SelectMultiTarget`
  (bind (_dragstartpos_x _dragstartpos_y) (`KismetMathLibrary.BreakVector2D` (`self.DragStartPos`)))
  (bind (_dragendpos_x _dragendpos_y) (`KismetMathLibrary.BreakVector2D` (`self.DragEndPos`)))
  (bind _outactors (`GameplayStatics.GetAllActorsOfClass` "/Game/MyGame/Blueprints/BP_ParentUnit.BP_ParentUnit_C"))
  (for _array_element _outactors
    (bind _asbp_parent_unit (cast `/Game/MyGame/Blueprints/BP_ParentUnit` _array_element))
    (bind _screenlocation (`self.ProjectWorldLocationToScreen` (`self.K2_GetActorLocation` _array_element) true))
    (if (and (> (`KismetMathLibrary.BreakVector2D` _screenlocation) (`KismetMathLibrary.FMin` _dragstartpos_x _dragendpos_x)) (< (`KismetMathLibrary.BreakVector2D` _screenlocation) (`KismetMathLibrary.FMax` _dragstartpos_x _dragendpos_x)) (> (`.Y` (`KismetMathLibrary.BreakVector2D` _screenlocation)) (`KismetMathLibrary.FMin` _dragstartpos_y _dragendpos_y)) (< (`.Y` (`KismetMathLibrary.BreakVector2D` _screenlocation)) (`KismetMathLibrary.FMax` _dragstartpos_y _dragendpos_y)) (== (`/Game/MyGame/Blueprints/BP_ParentUnit.TeamID` _asbp_parent_unit) 0))
      (`/Game/MyGame/Blueprints/BP_ParentUnit.Toggle Selection` _asbp_parent_unit true)
      (`KismetArrayLibrary.Array_AddUnique` (`self.MultiSelectUnits`) _asbp_parent_unit))))

(fn `SelectSingleTarget`
  (bind _asbp_parent_unit (cast `/Game/MyGame/Blueprints/BP_ParentUnit` (`.HitActor` (`GameplayStatics.BreakHitResult` (`self.GetHitResultUnderCursorByChannel` "TraceTypeQuery1")))))
  (if (== (`/Game/MyGame/Blueprints/BP_ParentUnit.TeamID` _asbp_parent_unit) 0)
    (bind _output_get (set `self.SelectedUnit` _asbp_parent_unit))
    (`/Game/MyGame/Blueprints/BP_ParentUnit.Toggle Selection` _output_get true)))

(fn `UserConstructionScript`)