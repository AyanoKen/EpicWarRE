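; Clickable castle on the conquest map that launches a battle when attacked.
; A click on a castle with non-zero AIType that connects to an AIType 0 castle stores its AI type, spawn data and ID in BP_GameInstance.
; It then shows a loading screen and opens TopDownMap after a short delay.
; ConsumeCastle sets CastleID and swaps the gold or steel material, resetting AIType only for gold.
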(event `self.ReceiveActorOnClicked`
  (params (ButtonPressed :type "Key Structure"))
  (if (!= (`self.AIType`) 0)
    (for _array_element (`self.ConnectedCastles`)
      (if (== (`/Game/MyGame/Blueprints/BP_ConquestCastle.AIType` _array_element) 0)
        (bind _asbp_game_instance (cast `/Game/MyGame/GameMode/BP_GameInstance` (`GameplayStatics.GetGameInstance`)))
        (set `/Game/MyGame/GameMode/BP_GameInstance.EnemyAIType` (`self.AIType`) _asbp_game_instance)
        (set `/Game/MyGame/GameMode/BP_GameInstance.EnemySpawnData` (`self.SpawnData`) _asbp_game_instance)
        (set `/Game/MyGame/GameMode/BP_GameInstance.ConquestTarget` (`self.CastleID`) _asbp_game_instance)
        (bind _returnvalue (`|CreateWidget` "/Game/MyGame/UI/WBP_LoadingScreen.WBP_LoadingScreen_C" (`GameplayStatics.GetPlayerController` 0)))
        (`UserWidget.AddToViewport` _returnvalue 0)
        (`KismetSystemLibrary.Delay` 0.5)
        (`GameplayStatics.OpenLevel` "TopDownMap")))))

(fn `ConsumeCastle`
  (params (ID :type Integer))
  (set `self.CastleID` ID)
  (switch `int` ID
    (:`0`
      (`PrimitiveComponent.SetMaterial` (`self.StaticMesh`) 0 "/Game/StarterContent/Materials/M_Metal_Gold.M_Metal_Gold")
      (set `self.AIType` 0))
    (:`1`
      (`PrimitiveComponent.SetMaterial` (`self.StaticMesh`) 0 "/Game/StarterContent/Materials/M_Metal_Steel.M_Metal_Steel"))))

(fn `UserConstructionScript`)