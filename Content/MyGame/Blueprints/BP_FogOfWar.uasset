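; BP_FogOfWar is a fog-of-war actor that toggles its own visibility based on which team 0 units are inside its box.
; Box begin and end overlap events add or remove those BP_ParentUnit actors in a CollidingUnits list, then call CheckVisibility.
; CheckVisibility shows the actor in game while the list has any units and hides it when the list is empty.
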(event `self.Box.OnComponentBeginOverlap`
  (params (OverlappedComponent :type "PrimitiveComponent Object Reference") (OtherActor :type "Actor Object Reference") (OtherComp :type "PrimitiveComponent Object Reference") (OtherBodyIndex :type Integer) (bFromSweep :type Boolean) (SweepResult :type "HitResult Structure (by ref)"))
  (bind _asbp_parent_unit (cast `/Game/MyGame/Blueprints/BP_ParentUnit` OtherActor))
  (if (== (`/Game/MyGame/Blueprints/BP_ParentUnit.TeamID` _asbp_parent_unit) 0)
    (`KismetArrayLibrary.Array_Add` (`self.CollidingUnits`) _asbp_parent_unit)
    (`self.CheckVisibility`)))

(event `self.Box.OnComponentEndOverlap`
  (params (OverlappedComponent :type "PrimitiveComponent Object Reference") (OtherActor :type "Actor Object Reference") (OtherComp :type "PrimitiveComponent Object Reference") (OtherBodyIndex :type Integer))
  (bind _asbp_parent_unit (cast `/Game/MyGame/Blueprints/BP_ParentUnit` OtherActor))
  (if (== (`/Game/MyGame/Blueprints/BP_ParentUnit.TeamID` _asbp_parent_unit) 0)
    (`KismetArrayLibrary.Array_RemoveItem` (`self.CollidingUnits`) _asbp_parent_unit)
    (`self.CheckVisibility`)))

(fn `CheckVisibility`
  (if (> (`KismetArrayLibrary.Array_Length` (`self.CollidingUnits`)) 0)
    (`self.SetActorHiddenInGame` false)
    (else
      (`self.SetActorHiddenInGame` true))))

(fn `UserConstructionScript`)