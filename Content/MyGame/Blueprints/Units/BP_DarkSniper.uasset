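; BP_DarkSniper is a bow-wielding unit Blueprint that adds an arrow effect to the attack logic inherited from its parent class.
; Its AttackLogic override runs the parent attack, then spawns the NS_Arrow2 Niagara system at the mesh's bow emitter socket.
; The effect is rotated toward the castle target when CastleAggro is set, otherwise toward the current target.
; The event graph and construction script add no logic of their own.
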(fn `AttackLogic`
  (bind _returnvalue (`SceneComponent.GetSocketLocation` (`self.Mesh`) "BowEmitterSocket"))
  (bind _returnvalue_2 (`SceneComponent.GetSocketLocation` (`self.Mesh`) "BowEmitterSocket"))
  (`parent.AttackLogic`)
  (if (not (`self.CastleAggro?`))
    (`NiagaraFunctionLibrary.SpawnSystemAtLocation` "/Game/MyGame/FX/NS_Arrow2.NS_Arrow2" _returnvalue_2 (`KismetMathLibrary.FindLookAtRotation` _returnvalue_2 (`self.K2_GetActorLocation` (`self.CurrentTarget`))))
    (else
      (`NiagaraFunctionLibrary.SpawnSystemAtLocation` "/Game/MyGame/FX/NS_Arrow2.NS_Arrow2" _returnvalue (`KismetMathLibrary.FindLookAtRotation` _returnvalue (`self.K2_GetActorLocation` (`self.CastleTarget`)))))))

(fn `UserConstructionScript`
  (`parent.UserConstructionScript`))