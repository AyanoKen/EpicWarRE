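; BP_Rogue is a unit Blueprint, apparently a bow-wielding ranged attacker, that adds an arrow effect to its parent's attack.
; Its AttackLogic override runs the parent logic, then spawns the NS_Arrow Niagara system at the mesh's BowEmitterSocket, rotated toward CurrentTarget's location.
; The event graph holds only disabled placeholder events, so all other behavior comes from the parent class.
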(fn `AttackLogic`
  (bind _returnvalue (`SceneComponent.GetSocketLocation` (`self.Mesh`) "BowEmitterSocket"))
  (`parent.AttackLogic`)
  (`NiagaraFunctionLibrary.SpawnSystemAtLocation` "/Game/MyGame/FX/NS_Arrow.NS_Arrow" _returnvalue (`KismetMathLibrary.FindLookAtRotation` _returnvalue (`self.K2_GetActorLocation` (`self.CurrentTarget`)))))

(fn `UserConstructionScript`
  (`parent.UserConstructionScript`))