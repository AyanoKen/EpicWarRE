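; BP_ParentUnit is the base team unit that moves, auto-fights enemy units and castles, and dies at zero HP.
; Detection overlaps maintain the target list and castle aggro, ignoring team 2 and same-team actors.
; TryAttack chases the first target with AIMoveTo, then loops montage, damage and cooldown through the empty AttackLogic hook, while castles are hit in place.
; One selection mesh shows both selection and health-tier materials.
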(event `self.DetectionCollider.OnComponentBeginOverlap`
  (params (OverlappedComponent :type "PrimitiveComponent Object Reference") (OtherActor :type "Actor Object Reference") (OtherComp :type "PrimitiveComponent Object Reference") (OtherBodyIndex :type Integer) (bFromSweep :type Boolean) (SweepResult :type "HitResult Structure (by ref)"))
  (bind _teamid (`self.TeamID`))
  (bind _teamid_2 (`self.TeamID`))
  ;[0.15 0.15 0.15 0.5 42] Detection Logic
  (bind _asbp_parent_unit (cast `/Game/MyGame/Blueprints/BP_ParentUnit` OtherActor)
    (:`then`
      (bind _teamid_3 (`/Game/MyGame/Blueprints/BP_ParentUnit.TeamID` _asbp_parent_unit))
      (if (not (or (== _teamid_2 2) (== _teamid_2 _teamid_3) (== _teamid_3 2)))
        (`KismetArrayLibrary.Array_Add` (`self.Targets`) _asbp_parent_unit)
        (if (not (`self.IsInBattle?`))
          (`self.TryAttack`))))
    (:`CastFailed`
      (bind _asbp_castle (cast `/Game/MyGame/Blueprints/BP_Castle` OtherActor))
      (bind _teamid_4 (`/Game/MyGame/Blueprints/BP_Castle.TeamId` _asbp_castle))
      (if (not (or (== _teamid 2) (== _teamid _teamid_4) (== _teamid_4 2)))
        (set `self.CastleAggro?` true)
        (set `self.CastleTarget` _asbp_castle)
        (`self.AttackCastle`)))))

(event `AttackCastle`
  (bind _castletarget (`self.CastleTarget`))
  ;[0.15 0.15 0.15 0.5 42] Attack Logic
  (if (and (`KismetSystemLibrary.IsValid` _castletarget) (not (`self.IsInBattle?`))) :!label _label
    (`self.PlayAnimMontage` (`self.AtkAnimation`))
    (`self.AttackLogic`)
    (`/Game/MyGame/Blueprints/BP_Castle.TakeDamage` _castletarget (`self.Damage`))
    (`KismetSystemLibrary.Delay` (`self.AtkCooldown`))
    (goto _label)))

(event `self.DetectionCollider.OnComponentEndOverlap`
  (params (OverlappedComponent :type "PrimitiveComponent Object Reference") (OtherActor :type "Actor Object Reference") (OtherComp :type "PrimitiveComponent Object Reference") (OtherBodyIndex :type Integer))
  ;[0.15 0.15 0.15 0.5 42] Detection Logic
  (bind _asbp_parent_unit (cast `/Game/MyGame/Blueprints/BP_ParentUnit` OtherActor)
    (:`then`
      (if (not (== (`/Game/MyGame/Blueprints/BP_ParentUnit.TeamID` _asbp_parent_unit) (`self.TeamID`)))
        (`KismetArrayLibrary.Array_RemoveItem` (`self.Targets`) _asbp_parent_unit)
        (if (== _asbp_parent_unit (`self.CurrentTarget`))
          (set `self.CurrentTarget` null))))
    (:`CastFailed`
      (bind _asbp_castle (cast `/Game/MyGame/Blueprints/BP_Castle` OtherActor))
      (if (not (== (`/Game/MyGame/Blueprints/BP_Castle.TeamId` _asbp_castle) (`self.TeamID`)))
        (set `self.CastleAggro?` false)
        (set `self.CastleTarget` null)))))

(event `TryAttack`
  (bind _targets (`self.Targets`))
  (bind _currenttarget (`self.CurrentTarget`))
  ;[0.15 0.15 0.15 0.5 42] Attack Logic
  (if (`self.CastleAggro?`)
    (`self.AttackCastle`)
    (elif (or (`self.IsInBattle?`) (`KismetArrayLibrary.Array_IsEmpty` _targets))
      _
      (elif (`self.CanAttack?`)
        (set `self.IsInBattle?` true)
        (set `self.CurrentTarget` (`|GetArrayItem` _targets))
        (`self.MoveToLocation` (`self.K2_GetActorLocation`))
        (if (`KismetSystemLibrary.IsValid` _currenttarget) :!label _label_2
          (`|AIMoveTo` self (0.0 0.0 0.0) _currenttarget (`self.AtkRange`)
            (:`then`
              (bind _returnvalue (`self.PlayAnimMontage` (`self.AtkAnimation`)))
              (`self.AttackLogic`)
              (`self.TakeDamage` _currenttarget self (`self.Damage`))
              (`KismetSystemLibrary.Delay` (+ _returnvalue (`self.AtkCooldown`)))
              (goto _label_2)))
          (else
            (set `self.CurrentTarget` null)
            (`KismetArrayLibrary.Array_Remove` (`self.Targets`))
            (set `self.IsInBattle?` false)
            (`self.TryAttack`)))
        (else
          (`KismetSystemLibrary.Delay` 1.0)
          (`self.TryAttack`))))))

(event `self.ReceiveBeginPlay`
  ;[0.15 0.15 0.15 0.5 42] BeginPlay
  (set `self.CurrentHp` (`self.MaxHp`)))

(event `Reposition`
  ;[0.15 0.15 0.15 0.5 42] Helper Functions
  (`self.MoveToLocation` (+ (* (`KismetMathLibrary.RotateAngleAxis` (`self.GetActorForwardVector`) (`KismetMathLibrary.RandomFloatInRange` -45.0 45.0) (0.0 0.0 1.0)) (`KismetMathLibrary.RandomFloatInRange` 200.0 400.0)) (`self.K2_GetActorLocation`))))

(event `TakeDamage`
  (params (Source :type "/Game/MyGame/Blueprints/BP_ParentUnit Object Reference") (Dmg :type Integer))
  ;[0.15 0.15 0.15 0.5 42] Take Damage
  (if (> (`self.CurrentHp`) 0)
    (bind _output_get (set `self.CurrentHp` (- (`self.CurrentHp`) Dmg)))
    (if (<= _output_get 0)
      (bind _returnvalue (`self.PlayAnimMontage` (`self.DeathAnimation`)))
      (`KismetSystemLibrary.Delay` _returnvalue)
      (`self.K2_DestroyActor`)
      (else
        (`self.SetHpIndicator`)))))

(fn `AttackLogic`)

(fn `ChangeHpIndicator`
  (if (!= (`self.TeamID`) 0)
    (`StaticMeshComponent.SetStaticMesh` (`self.SelectionUI`) "/Game/MyGame/Meshes/Cross.Cross")))

(fn `MoveToLocation`
  (params (Destination :type "Vector Structure"))
  (bind _asaicontroller (cast `AIController` (`self.GetController` self)))
  (`AIController.MoveToLocation` _asaicontroller Destination -1.0 true true false true null true)
  (`self.TryAttack`))

(fn `SetHpIndicator`
  (if (<= (/ (`KismetMathLibrary.Conv_IntToDouble` (`self.CurrentHp`)) (`KismetMathLibrary.Conv_IntToDouble` (`self.MaxHp`))) 0.25)
    (`PrimitiveComponent.SetMaterial` (`self.SelectionUI`) 0 "/Game/MyGame/Materials/M_LowHP.M_LowHP")
    (elif (<= (/ (`KismetMathLibrary.Conv_IntToDouble` (`self.CurrentHp`)) (`KismetMathLibrary.Conv_IntToDouble` (`self.MaxHp`))) 0.75)
      (`PrimitiveComponent.SetMaterial` (`self.SelectionUI`) 0 "/Game/MyGame/Materials/M_MidHP.M_MidHP")
      (else
        (`PrimitiveComponent.SetMaterial` (`self.SelectionUI`) 0 "/Game/MyGame/Materials/M_FullHP.M_FullHP")))))

(fn `Toggle Selection`
  (params (`Enable?` :type Boolean))
  (bind _output_get (set `self.IsSelected?` `Enable?`))
  (if _output_get
    (`PrimitiveComponent.SetMaterial` (`self.SelectionUI`) 0 "/Game/MyGame/Materials/M_SelectionRing.M_SelectionRing")
    (else
      (`self.SetHpIndicator`))))

(fn `UserConstructionScript`)